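; My_PC is the player controller: it shows the cursor in game-only input mode, displays a debug HUD and manages the inventory screens.
; When CommenceJeu is set, BeginPlay disables My_Player input, plays a timed sleeping flipbook sequence, then restores idle animation and input.
; The I key flip-flops the inventory and selection-menu widgets on and off the viewport, creating each once and reusing it.
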(event `self.ReceiveBeginPlay`
  (set `self.bShowMouseCursor` true)
  (`WidgetBlueprintLibrary.SetInputMode_GameOnly` self)
  (`|ExecutionSequence`
    (:`then_0`
      (`self.HUD - DEBUG`))
    (:`then_1`
      (if (`self.CommenceJeu`)
        (bind _asmy_player (cast `/Game/Blueprints/My_Player` (`GameplayStatics.GetPlayerCharacter` 0)))
        (`self.DisableInput` _asmy_player self)
        (bind _sprite (`PaperCharacter.Sprite` _asmy_player))
        (`PaperFlipbookComponent.SetFlipbook` _sprite "/Game/Data/img/Hero_FB_Sleep.Hero_FB_Sleep")
        (`KismetSystemLibrary.Delay` 4.2)
        (`PaperFlipbookComponent.Stop` _sprite)
        (`KismetSystemLibrary.Delay` 2.0)
        (`PaperFlipbookComponent.SetFlipbook` _sprite "/Game/Data/img/Hero_FB_IDLE.Hero_FB_IDLE")
        (`self.EnableInput` _asmy_player self)
        (`PaperFlipbookComponent.Play` _sprite)))))

(event `Key|I`
  (params (Key :type "Key Structure"))
  (:`Pressed`
    (`/Engine/EditorBlueprintResources/StandardMacros.FlipFlop`
      (:`A`
        (`self.HUD - Inventaire`)
        (`self.HUD_SelectMenuInventaire`))
      (:`B`
        (`Widget.RemoveFromParent` (`self.HUD_Inventaire`))
        (`Widget.RemoveFromParent` (`self.HUD_SelectMenuInv`))))))

(event `HUD - Inventaire`
  (`/Engine/EditorBlueprintResources/StandardMacros.IsValid` (`self.HUD_Inventaire`)
    (:`Is Valid`
      _)
    (:`Is Not Valid`
      (bind _returnvalue (`|CreateWidget` "/Game/HUD/HUD_Inventaire.HUD_Inventaire_C"))
      (bind _output_get (set `self.HUD_Inventaire` _returnvalue))))
  (`UserWidget.AddToViewport` _output_get 0))

(event `HUD - DEBUG`
  (`/Engine/EditorBlueprintResources/StandardMacros.IsValid` (`self.HUD_Debug`)
    (:`Is Valid`
      _)
    (:`Is Not Valid`
      (bind _returnvalue (`|CreateWidget` "/Game/HUD/HUD_DEBUG.HUD_DEBUG_C"))
      (bind _output_get (set `self.HUD_Debug` _returnvalue))))
  (`UserWidget.AddToViewport` _output_get 0))

(event `HUD_SelectMenuInventaire`
  (`/Engine/EditorBlueprintResources/StandardMacros.IsValid` (`self.HUD_SelectMenuInv`)
    (:`Is Valid`
      _)
    (:`Is Not Valid`
      (bind _returnvalue (`|CreateWidget` "/Game/HUD/HUD_SelectionMenuInventaire.HUD_SelectionMenuInventaire_C"))
      (bind _output_get (set `self.HUD_SelectMenuInv` _returnvalue))))
  (`UserWidget.AddToViewport` _output_get 0))

(fn `UserConstructionScript`)