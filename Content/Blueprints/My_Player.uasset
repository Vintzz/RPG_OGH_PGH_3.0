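; Player character with a flipbook sprite, showing the player controller's name in a text render, with mouse-wheel spring arm zoom.
; Axis inputs move it and feed Movement, which plays a walk camera shake, rotates the sprite left or right and switches run/idle, idling only on specific frames.
; PrendCoup starts a looping timer that interpolates the capsule along Y as knockback, cleared after a delay.
; The attack animation and stop-wait chains are unconnected.
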(event `self.ReceiveBeginPlay`
  (`SceneComponent.K2_SetRelativeRotation` (`self.CapsuleComponent`) (struct :`Pitch` 70.0) false false)
  (bind _asmy_pc (cast `/Game/Blueprints/My_PC` (`GameplayStatics.GetPlayerController` 0)))
  (`TextRenderComponent.K2_SetText` (`self.TextRender`) (`/Game/Blueprints/My_PC.PlayerName` _asmy_pc)))

(event `InputAxis|Keyboard Up Down`
  (params (AxisValue :type "Float (single-precision)"))
  (`self.AddMovementInput` (`KismetMathLibrary.MakeVector` (`self.VitesseDeplacement`)) (* AxisValue -1.0))
  (`self.Movement` AxisValue))

(event `InputAxis|Keyboard Left Right`
  (params (AxisValue :type "Float (single-precision)"))
  (`self.AddMovementInput` (`KismetMathLibrary.MakeVector` 0.0 (`self.VitesseDeplacement`)) (* AxisValue -1.0))
  (`self.Movement` AxisValue))

(event `Movement`
  (params (Scale :type "Float (double-precision)"))
  (bind _returnvalue (`PaperFlipbookComponent.GetPlaybackPositionInFrames` (`self.Sprite`)))
  (`|ExecutionSequence`
    (:`then_0`
      (if (> (`KismetMathLibrary.VSize` (`self.GetVelocity`)) 0.0)
        (`self.SetFlipBook` 1)))
    (:`then_1`
      (`PlayerController.ClientStartCameraShake` :`self` (`GameplayStatics.GetPlayerController` 0) :`Shake` "/Game/Blueprints/CS_Walk.CS_Walk_C" :`Scale` (`KismetMathLibrary.Square` Scale)))
    (:`then_2`
      (`/Engine/EditorBlueprintResources/StandardMacros.CompareFloat` (* Scale -1.0)
        (:`>`
          (`self.SetRotation` "NewEnumerator1"))
        (:`==`
          (if (and (or (== _returnvalue 2) (== _returnvalue 6)) (<= (`KismetMathLibrary.VSize` (`self.GetVelocity`)) 0.0))
            (`self.SetFlipBook` 0)))
        (:`<`
          (`self.SetRotation` "NewEnumerator0"))))))

(event `InputAction|Base Attack`
  (params (Key :type "Key Structure")))

(event `WaitStopAnim`
  (bind _returnvalue (`PaperFlipbookComponent.GetPlaybackPositionInFrames` (`self.Sprite`)))
  (if (or (== _returnvalue 0) (== _returnvalue 4))
    _))

(event `Key|MouseScrollUp`
  (params (Key :type "Key Structure"))
  (bind _springarm (`self.SpringArm`))
  (bind _targetarmlength (`SpringArmComponent.TargetArmLength` _springarm))
  (:`Pressed`
    (if (> _targetarmlength (`self.ZoomMin`))
      (set `SpringArmComponent.TargetArmLength` (- _targetarmlength 100.0) _springarm))))

(event `Key|MouseScrollDown`
  (params (Key :type "Key Structure"))
  (bind _springarm (`self.SpringArm`))
  (bind _targetarmlength (`SpringArmComponent.TargetArmLength` _springarm))
  (:`Pressed`
    (if (< _targetarmlength (`self.ZoomMax`))
      (set `SpringArmComponent.TargetArmLength` (+ _targetarmlength 100.0) _springarm))))

(event `PrendCoup`
  (params (Direction :type Integer))
  (switch `int` Direction
    (:`0`
      (set `self.XForceMov` -10.0))
    (:`1`
      (set `self.XForceMov` 10.0)))
  (bind _returnvalue (`KismetSystemLibrary.K2_SetTimerDelegate` (delegate `PrendCoup - Move`) 0.01 true)))

(event `PrendCoup - Move`
  (bind _capsulecomponent (`self.CapsuleComponent`))
  (bind (_returnvalue_x _returnvalue_y _returnvalue_z) (`KismetMathLibrary.BreakVector` (`SceneComponent.K2_GetComponentLocation` _capsulecomponent)))
  (`SceneComponent.K2_SetWorldLocation` _capsulecomponent (`KismetMathLibrary.VInterpTo` (`SceneComponent.K2_GetComponentLocation` _capsulecomponent) (`KismetMathLibrary.MakeVector` _returnvalue_x (+ _returnvalue_y (`self.XForceMov`)) _returnvalue_z) (`GameplayStatics.GetWorldDeltaSeconds`) 3.0) false false)
  (`KismetSystemLibrary.Delay` 0.5)
  (`KismetSystemLibrary.K2_ClearAndInvalidateTimerHandle` (stale `PrendCoup` _returnvalue)))

(fn `SetFlipBook`
  (params (FB :type Integer))
  (`PaperFlipbookComponent.SetFlipbook` (`self.Sprite`) (select `int` FB :`0` "/Game/Data/img/Hero_FB_IDLE.Hero_FB_IDLE" :`1` "/Game/Data/img/Hero_FB_RUN.Hero_FB_RUN" :`2` "/Game/Data/img/Hero_FB_Tappe.Hero_FB_Tappe" :`3` null :`4` null :!type "PaperFlipbook Object Reference")))

(fn `SetRotation`
  (params (Rotation :type "/Game/Blueprints/Player_Rot Enum" :default "NewEnumerator0"))
  (bind _sprite (`self.Sprite`))
  (switch `/Game/Blueprints/Player_Rot` Rotation
    (:`NewEnumerator0`
      (`SceneComponent.K2_SetRelativeRotation` _sprite (struct :`Yaw` -90.0) false false))
    (:`NewEnumerator1`
      (`SceneComponent.K2_SetRelativeRotation` _sprite (struct :`Yaw` 90.0) false false))))

(fn `UserConstructionScript`)