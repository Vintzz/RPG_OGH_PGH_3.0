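; Player pawn for a top-down game with a Paper2D flipbook hero that walks, attacks and zooms its camera.
; Axis input offsets the actor in world space, rotates the sprite to face left or right, and switches between run and idle flipbooks.
; Attacking locks movement, polls on a looping timer for a specific animation frame, then plays the hit flipbook before unlocking.
; Mouse wheel changes spring arm length within zoom limits.
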(event `self.ReceiveBeginPlay`
  (`SceneComponent.K2_SetRelativeRotation` (`self.Hero`) (struct :`Yaw` -90.0 :`Roll` -70.0) false false)
  (`SceneComponent.K2_SetRelativeRotation` (`self.SpringArm`) (struct :`Pitch` -70.0 :`Yaw` 180.0) false false))

(event `InputAxis|Keyboard Up Down`
  (params (AxisValue :type "Float (single-precision)"))
  (if (and (`self.CanMove`) true)
    (set `self.AxisUD` AxisValue)
    (if (== AxisValue 1.0)
      (`self.K2_AddActorWorldOffset` (`KismetMathLibrary.MakeVector` 0.0 (`self.VitesseDeplacement`)))
      (`self.Movement Player` :!label _label)
      (elif (== AxisValue -1.0)
        (`self.K2_AddActorWorldOffset` (`KismetMathLibrary.MakeVector` 0.0 (* (`self.VitesseDeplacement`) -1.0)))
        (goto _label)
        (elif (and (== AxisValue 0.0) (== (`self.AxisRL`) 0.0))
          (`PaperFlipbookComponent.SetFlipbook` (`self.Hero`) "/Game/Data/img/Hero_FB_IDLE.Hero_FB_IDLE"))))))

(event `InputAxis|Keyboard Left Right`
  (params (AxisValue :type "Float (single-precision)"))
  (bind _hero (`self.Hero`))
  (if (and (`self.CanMove`) true)
    (set `self.AxisRL` AxisValue)
    (if (== AxisValue 1.0)
      (`self.K2_AddActorWorldOffset` (`KismetMathLibrary.MakeVector` (* (`self.VitesseDeplacement`) -1.0)))
      (`SceneComponent.K2_SetRelativeRotation` _hero (struct :`Yaw` -90.0 :`Roll` -70.0) false false)
      (`self.Movement Player` :!label _label_2)
      (elif (== AxisValue -1.0)
        (`self.K2_AddActorWorldOffset` (`KismetMathLibrary.MakeVector` (`self.VitesseDeplacement`)))
        (`SceneComponent.K2_SetRelativeRotation` _hero (struct :`Yaw` 90.0 :`Roll` 70.0) false false)
        (goto _label_2)
        (elif (and (== AxisValue 0.0) (== (`self.AxisUD`) 0.0))
          (`PaperFlipbookComponent.SetFlipbook` (`self.Hero`) "/Game/Data/img/Hero_FB_IDLE.Hero_FB_IDLE"))))))

(event `InputAction|Base Attack`
  (params (Key :type "Key Structure"))
  (:`Pressed`
    (set `self.CanMove` false)
    (bind _returnvalue (`KismetSystemLibrary.K2_SetTimerDelegate` (delegate `WaitStopAnim`) 0.01 true))))

(event `WaitStopAnim`
  (bind _returnvalue (`PaperFlipbookComponent.GetPlaybackPositionInFrames` (`self.Hero`)))
  (if (or (== _returnvalue 0) (== _returnvalue 4))
    (`KismetSystemLibrary.K2_ClearAndInvalidateTimerHandle` (stale `InputAction|Base Attack` _returnvalue))
    (`PaperFlipbookComponent.SetFlipbook` (`self.Hero`) "/Game/Data/img/Hero_FB_Tappe.Hero_FB_Tappe")
    (`KismetSystemLibrary.Delay` 0.5)
    (set `self.CanMove` true)))

(event `Key|MouseScrollUp`
  (params (Key :type "Key Structure"))
  (bind _springarm (`self.SpringArm`))
  (bind _targetarmlength (`SpringArmComponent.TargetArmLength` _springarm))
  (:`Pressed`
    (if (> _targetarmlength (`self.ZoomMin`))
      (set `SpringArmComponent.TargetArmLength` (- _targetarmlength 100.0) _springarm))))

(event `Key|MouseScrollDown`
  (params (Key :type "Key Structure"))
  (bind _springarm (`self.SpringArm`))
  (bind _targetarmlength (`SpringArmComponent.TargetArmLength` _springarm))
  (:`Pressed`
    (if (< _targetarmlength (`self.ZoomMax`))
      (set `SpringArmComponent.TargetArmLength` (+ _targetarmlength 100.0) _springarm))))

(fn `UserConstructionScript`)