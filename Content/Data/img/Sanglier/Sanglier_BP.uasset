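; Boar (Sanglier) pawn that wanders randomly around the navigable area.
; After a random delay at BeginPlay, it uses AIMoveTo toward a random navigable point within a radius of its current location.
; Success and failure both lead to another random pause and a new move, forming an endless loop.
; The capsule component's relative rotation is forced to a fixed value at BeginPlay and every Tick.
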(event `self.ReceiveTick`
  (params (DeltaSeconds :type "Float (single-precision)"))
  (`SceneComponent.K2_SetRelativeRotation` (`self.CapsuleComponent`) (struct :`Pitch` 70.0) false false))

(event `self.ReceiveBeginPlay`
  (`SceneComponent.K2_SetRelativeRotation` (`self.CapsuleComponent`) (struct :`Pitch` 70.0) false false)
  (`KismetSystemLibrary.Delay` (`KismetMathLibrary.RandomFloatInRange` 5.0 10.0))
  (`self.MoveRandomPos`))

(event `MoveRandomPos`
  (`|AIMoveTo` self (`NavigationSystem.K2_GetRandomLocationInNavigableRadius` (`self.K2_GetActorLocation`) 1000.0)
    (:`OnSuccess`
      _)
    (:`OnFail`
      _))
  (`KismetSystemLibrary.Delay` (`KismetMathLibrary.RandomFloatInRange` 5.0 10.0))
  (`self.MoveRandomPos`))

(fn `UserConstructionScript`)